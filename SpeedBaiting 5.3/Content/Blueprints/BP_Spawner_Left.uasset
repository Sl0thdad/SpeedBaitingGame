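; BP_Spawner_Left is a note spawner that emits BP_Beat_Left actors at its own transform following a pattern.
; The Map array holds run lengths that alternately toggle SendNote between silence and notes.
; Tick feeds a Delay, so each step counts down the current run and spawns a beat while SendNote is true.
; Exhausted runs advance immediately to the next entry, and spawning stops after the last.
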(event EventBeginPlay
  (Variables|Default|SetCount (Utilities|Array|Get(acopy) (Variables|Default|GetMap))))

(event EventTick
  (params (DeltaSeconds :type Float%20%28single-precision%29))
  (bind _map (Variables|Default|GetMap))
  (bind _index (Variables|Default|GetIndex))
  (Utilities|FlowControl|Delay (Variables|Default|GetDelay))
  (Math|Integer|DecrementInt (Variables|Default|GetCount) :!label _label
    (:%20%20
      (if (== (Variables|Default|GetCount) -1)
        (if (== _index (- (Utilities|Array|Length _map) 1))
          (Variables|Default|SetSendNote false)
          (else
            (Math|Integer|IncrementInt _index
              (:%20%20
                (Variables|Default|SetCount (Utilities|Array|Get(acopy) _map (Variables|Default|GetIndex)))
                (Variables|Default|SetSendNote (not (Variables|Default|GetSendNote)))
                (goto _label))))))
      (if (Variables|Default|GetSendNote)
        (Game|SpawnActorfromClass "/Game/Blueprints/BP_Beat_Left.BP_Beat_Left_C" (Transformation|GetActorTransform) "Undefined" "MultiplyWithRoot" 0 0)))))

(fn ConstructionScript)