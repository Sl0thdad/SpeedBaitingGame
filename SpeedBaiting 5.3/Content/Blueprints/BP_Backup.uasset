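; BP_Backup is a key-timed hit-detection prototype with two capsule zones, each tracking whether something overlaps it.
; Begin and end overlap events set a flag per capsule, which X checks for Capsule1 and Z for Capsule2, printing hit or miss.
; A Z hit also destroys OtherActor, a value supplied only by Capsule1's begin-overlap event.
; BeginPlay shows the mouse cursor.
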(event OnComponentBeginOverlap(Capsule2)
  (params (OverlappedComponent :type Primitive%20Component%20Object%20Reference) (OtherActor :type Actor%20Object%20Reference) (OtherComp :type Primitive%20Component%20Object%20Reference) (OtherBodyIndex :type Integer) (bFromSweep :type Boolean) (SweepResult :type Hit%20Result%20Structure%20%28by%20ref%29))
  (Variables|Default|SetOverlap%20Cap2 true)
  (Development|PrintString "Overlap2"))

(event OnComponentEndOverlap(Capsule2)
  (params (OverlappedComponent :type Primitive%20Component%20Object%20Reference) (OtherActor :type Actor%20Object%20Reference) (OtherComp :type Primitive%20Component%20Object%20Reference) (OtherBodyIndex :type Integer))
  (Variables|Default|SetOverlap%20Cap2 false))

(event OnComponentBeginOverlap(Capsule1)
  (params (OverlappedComponent :type Primitive%20Component%20Object%20Reference) (OtherActor :type Actor%20Object%20Reference) (OtherComp :type Primitive%20Component%20Object%20Reference) (OtherBodyIndex :type Integer) (bFromSweep :type Boolean) (SweepResult :type Hit%20Result%20Structure%20%28by%20ref%29))
  (Variables|Default|SetOverlap%20Cap1 true)
  (Development|PrintString (Utilities|GetDisplayName OtherActor)))

(event OnComponentEndOverlap(Capsule1)
  (params (OverlappedComponent :type Primitive%20Component%20Object%20Reference) (OtherActor :type Actor%20Object%20Reference) (OtherComp :type Primitive%20Component%20Object%20Reference) (OtherBodyIndex :type Integer))
  (Variables|Default|SetOverlap%20Cap1 false))

(event EventBeginPlay
  (Variables|/Script/Engine.PlayerController|SetbShowMouseCursor (Game|GetPlayerController 0) true))

(event Input|KeyboardEvents|Z
  (params (Key :type Key%20Structure :default "None"))
  (:Pressed
    (if (Variables|Default|GetOverlap%20Cap2)
      (Development|PrintString "Hit2")
      (Actor|DestroyActor (stale OnComponentBeginOverlap(Capsule1) OtherActor))
      (else
        (Development|PrintString "Miss2")))))

(event Input|KeyboardEvents|X
  (params (Key :type Key%20Structure :default "None"))
  (:Pressed
    (if (Variables|Default|GetOverlap%20Cap1)
      (Development|PrintString "Hit1")
      (else
        (Development|PrintString "miss1")))))

(fn ConstructionScript)