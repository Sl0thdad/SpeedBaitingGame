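; BP_Beat is a clickable beat actor that travels from its starting position toward a relative Destination offset.
; The construction script stores the start location and adds it and the offset as InterpToMovement control points.
; Clicking the actor prints a debug "Hello" and destroys it.
; Tick also destroys it, without printing, once its location is within a small tolerance of the end point.
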(event EventTick
  (params (DeltaSeconds :type Float%20%28single-precision%29))
  (if (Utilities|Operators|EqualEqual (Transformation|GetActorLocation) (+ (Variables|Default|GetStartPos) (Variables|Default|GetDestination)) 0.5)
    (Actor|DestroyActor)))

(event MouseInput|EventActorOnClicked
  (params (ButtonPressed :type Key%20Structure :default "None"))
  (Development|PrintString "Hello")
  (Actor|DestroyActor))

(fn ConstructionScript
  (bind _output_get (Variables|Default|SetStartPos (Transformation|GetActorLocation)))
  (Class|InterptoMovementComponent|AddControlPointPosition (Variables|Default|GetInterpToMovement) _output_get false)
  (Class|InterptoMovementComponent|AddControlPointPosition (Variables|Default|GetInterpToMovement) (Variables|Default|GetDestination) true))